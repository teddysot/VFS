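; Test player controller that forwards movement and jump input to the pawn it controls.
; Every tick it builds a world-space vector from the Vertical and Horizontal values and adds it as movement input, independent of camera or control rotation.
; The Jump action calls Jump on the pawn through a CastToTestPlayerPawn helper, so it only acts when that pawn is a TestPlayerPawn.
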(event EventBeginPlay)

(event EventTick
  (params (DeltaSeconds :type Float%20%28single-precision%29))
  (Pawn|Input|AddMovementInput (Pawn|GetControlledPawn) (Math|Vector|MakeVector (Input|AxisValues|GetVertical) (Input|AxisValues|GetHorizontal) 0.0) 1.0 false))

(event Input|ActionEvents|InputActionJump
  (params (Key :type Key%20Structure))
  ;[1 1 1] Send jump input to controlled pawn
  (:Pressed
    (bind _astest_player_pawn (Utilities|CasttoTestPlayerPawn)
      (:Success
        (Default|Jump _astest_player_pawn 1.0)))))

(fn ConstructionScript)