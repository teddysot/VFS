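; Weapon component that fires projectiles at a limited rate.
; TryShoot compares real time against NextFireTime and, once the cooldown has elapsed, sets the next allowed time and calls Fire.
; Fire spawns the Projectile class at the transform of the supplied Arrow, ignoring collisions, and plays the player weapon sound at that location.
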(event Custom|TryShoot
  (params (Arrow :type Arrow%20Component%20Object%20Reference))
  ;[1 1 1] Checks if we can fire
  (Math|Float|CompareFloat (Utilities|Time|GetRealTimeSeconds) (Variables|Default|Get_nextFireTime)
    (:>
      _)
    (:==
      _))
  (Variables|Default|Set_nextFireTime (+ (Utilities|Time|GetRealTimeSeconds) (Variables|Default|Get_coolDown)))
  ;[1 1 1] Actually fire
  (CallFunction|Fire Arrow))

(event Custom|Fire
  (params (Arrow :type Arrow%20Component%20Object%20Reference))
  (bind _returnvalue (Transformation|GetWorldTransform Arrow))
  ;[1 1 1] Fire weapon
  (Game|SpawnActorfromClass (Variables|Default|Get_projectile) _returnvalue "AlwaysSpawn" 0 0)
  (Audio|PlaySoundatLocation "/Game/Audio/weapon_player.weapon_player" (.Location (Math|Transform|BreakTransform _returnvalue)) "0, 0, 0" 1.0 1.0 0.0 0 0 0))