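; Health actor component that tracks its owner's health and signals death.
; BeginPlay copies the starting CurrentHealth into MaxHealth, and the Damage event subtracts an amount from CurrentHealth.
; Tick polls CurrentHealth every frame and calls the death event whenever it is at or below zero, with no guard against repeat calls.
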(event Custom|Damage
  (params (Amount :type Float%20%28single-precision%29))
  ;[1 1 1] Damage Health
  (Variables|Default|Set_currentHealth (- (Variables|Default|Get_currentHealth) Amount)))

(event EventBeginPlay
  (Variables|Default|Set_maxHealth (Variables|Default|Get_currentHealth)))

(event EventTick
  (params (DeltaSeconds :type Float%20%28single-precision%29))
  ;[1 1 1] Check for death
  (if (<= (Variables|Default|Get_currentHealth) 0.0)
    (Default|CallDeathEvent)))