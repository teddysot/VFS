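; AOE actor component that fires an area burst of bullets around the player from a supplied Arrow.
; Its Fire event loops over ShotCount, spawning each bullet at the Arrow's location with its rotation combined with a yaw offset.
; That offset, HalfAngle, grows by a random step after every shot and is not reset here, giving uneven spacing.
; One explosion sound plays at the Arrow after the loop.
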(event EventFire
  (params (Arrow :type Arrow%20Component%20Object%20Reference))
  (Variables|Default|Set_arrow Arrow)
  (for _index (range 0 (Variables|Default|Get_shotCount))
    ;[1 1 1] Spawn bullet
    (Game|SpawnActorfromClass "/Game/Blueprints/Actors/Bullet.Bullet_C" (Math|Transform|MakeTransform (Transformation|GetWorldLocation (Variables|Default|Get_arrow)) (Math|Rotator|CombineRotators (Math|Rotator|MakeRotator 0.0 0.0 (stale _output_get)) (Transformation|GetWorldRotation (Variables|Default|Get_arrow))) "1,1,1") "Undefined" 0 0)
    ;[1 1 1] Create spawn point around player
    (bind _output_get (Variables|Default|Set_halfAngle (+ (Variables|Default|Get_halfAngle) (Math|Random|RandomFloatinRange 15.0 6e+01)))))
  ;[1 1 1] Play fire sound
  (Audio|PlaySoundatLocation "/Game/Audio/explosion_player.explosion_player" (Transformation|GetWorldLocation (Variables|Default|Get_arrow)) "0, 0, 0" 1.0 1.0 0.0 0 0 0))