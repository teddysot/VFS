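; Player ship actor that flies by physics, takes damage and cycles between Blaster, Shotgun and AOE weapons.
; Each tick, consumed movement input becomes forward force and yaw torque on the Ship.
; Damage feeds the Health component, whose death event hides the ship, disables its collision responses and shows the GameOver screen.
; BeginPlay also initializes DamageOnCollision and creates the health bar; firing requires health above zero.
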(event Custom|OnDeath
  ;[1 1 1] Set up Health
  (Rendering|SetVisibility (Variables|Default|GetShip) false false)
  (Collision|SetCollisionResponsetoAllChannels (Variables|Default|GetShip) "ECR_Ignore")
  ;[1 1 1] Create GameOver screen
  (bind _returnvalue (UserInterface|CreateWidget "/Game/Blueprints/Widgets/GameOver.GameOver_C"))
  (UserInterface|Viewport|AddtoViewport _returnvalue 0))

(event Custom|TryShoot
  ;[1 1 1] Shoot weapon
  (Math|Float|CompareFloat (Variables|/Game/Blueprints/ActorComponents/Health.Health_C|Get_currentHealth (Variables|Default|GetHealth)) 0.0
    (:>
      (Default|TryShoot (Utilities|Array|Get(acopy) (Variables|Default|Get_weapons) (Variables|Default|Get_weaponIndex)) (Variables|Default|GetArrow)))))

(event Custom|ChangeWeapon
  ;[1 1 1] Change weapon
  (bind _result (Math|Integer|IncrementInt (Variables|Default|Get_weaponIndex))
    (:%20%20
      (Math|Integer|CompareInt _result (Utilities|Array|Length (Variables|Default|Get_weapons))
        (:>
          _)
        (:==
          _))
      (Variables|Default|Set_weaponIndex 0))))

(event EventBeginPlay
  ;[1 1 1] Set up to DamageOnCollision
  (Default|Initialize (Variables|Default|GetDamageOnCollision) (Variables|Default|GetShip))
  ;[1 1 1] Set up Health
  (EventDispatchers|BindEventtoDeathEvent (Variables|Default|GetHealth) (delegate Custom|OnDeath))
  ;[1 1 1] Set up HUD
  (bind _returnvalue (UserInterface|CreateWidget "/Game/Blueprints/Widgets/HealthBar.Healthbar_C"))
  (UserInterface|Viewport|AddtoViewport _returnvalue 0)
  ;[1 1 1] Make weapons array
  (Variables|Default|Set_weapons (Utilities|Array|MakeArray (Variables|Default|GetBlaster) (Variables|Default|GetShotgun) (Variables|Default|GetAOE))))

(event Game|Damage|EventAnyDamage
  (params (Damage :type Float%20%28single-precision%29) (DamageType :type Damage%20Type%20Object%20Reference) (InstigatedBy :type Controller%20Object%20Reference) (DamageCauser :type Actor%20Object%20Reference))
  ;[1 1 1] Take damage
  (Default|Damage (Variables|Default|GetHealth) Damage))

(event EventTick
  (params (DeltaSeconds :type Float%20%28single-precision%29))
  (CallFunction|HandleMovement))

(fn ConstructionScript)

(fn HandleMovement
  (bind _ship (Variables|Default|GetShip))
  (bind _ship_2 (Variables|Default|GetShip))
  (bind _returnvalue (Class|Pawn|ConsumeMovementInputVector))
  ;[1 1 1] Up/Down Movement
  (Physics|AddForce _ship (* (* (Math|Vector|GetForwardVector _ship) (.y _returnvalue)) (Variables|Default|Get_moveSpeed)) "None" false)
  ;[1 1 1] Rotate Movement
  (Class|PrimitiveComponent|AddTorqueinDegrees _ship_2 (* (* (Math|Vector|GetUpVector _ship_2) (.x _returnvalue)) (Variables|Default|Get_turnSpeed)) "None" false))