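; Bullet is a projectile actor that can take damage and be destroyed.
; On BeginPlay it passes its sphere to Projectile for launch and to DamageOnCollision for setup, and binds Health's death event to destroy the actor.
; Any damage received is forwarded to Health.
; An experimental rotation lerp at launch uses full alpha, so it applies a one-time yaw offset instead of animating.
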(event Custom|OnDeath
  ;[1 1 1] Set up Health
  (Actor|DestroyActor))

(event EventBeginPlay
  (bind _returnvalue (Transformation|GetActorRotation))
  ;[1 1 1] Set up projectile
  (Default|Launch (Variables|Default|GetProjectile) (Variables|Default|GetSphere))
  ;[1 1 1] Set up to DamageOnCollision
  (Default|Initialize (Variables|Default|GetDamageOnCollision) (Variables|Default|GetSphere))
  ;[1 1 1] Set up Health
  (EventDispatchers|BindEventtoDeathEvent (Variables|Default|GetHealth) (delegate Custom|OnDeath))
  (Transformation|SetActorRotation (Math|Rotator|Lerp(Rotator) (Transformation|GetActorRotation) (Math|Rotator|MakeRotator (.roll _returnvalue) (.pitch _returnvalue) (+ (.yaw _returnvalue) 1e+03)) 1.0)))

(event Game|Damage|EventAnyDamage
  (params (Damage :type Float%20%28single-precision%29) (DamageType :type Damage%20Type%20Object%20Reference) (InstigatedBy :type Controller%20Object%20Reference) (DamageCauser :type Actor%20Object%20Reference))
  ;[1 1 1] Take damage
  (Default|Damage (Variables|Default|GetHealth) Damage))

(fn ConstructionScript)